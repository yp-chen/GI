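; Game mode for a gizmo-based model editing scene, handling light editing, model clearing and screenshot saving.
; Clicking a light shows or hides the adjustment widget and syncs its sliders; helper functions apply intensity, color and radius to the actor's point light components.
; Clearing destroys all target static meshes and hides the gizmo.
; Screen capture deselects the gizmo, waits briefly, exports a render target as a named PNG and reimports it as a texture.
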(event Custom|clickLight
  (params (Inclick :type Integer) (ClickedActor :type Actor%20Object%20Reference))
  (bind _w_lightadjust (Variables|Default|GetW_LIghtAdjust))
  (bind _output_get (Variables|Default|SetInclick Inclick))
  (switch int _output_get
    (:0
      (CallFunction|Hidewidget _w_lightadjust))
    (:1
      (CallFunction|ShowWidget _w_lightadjust :!label _label)
      (Variables|Default|SetCurrentLightActor ClickedActor))
    (:2
      (goto _label)))
  (Variables|Default|SetClickedActor ClickedActor)
  (CallFunction|SetLightSliderValue))

(event Custom|ScreenCut
  (bind _returnvalue (Class|BlueprintPathsLibrary|ProjectSavedDir))
  (bind _savename (Variables|Default|GetsaveName))
  (bind _returnvalue_2 (Utilities|String|ToString(Text) _savename))
  (bind _returnvalue_3 (Utilities|String|Append _returnvalue "SaveGames/Screenshots/"))
  (bind _returnvalue_4 (Utilities|String|Append _returnvalue_2 ".png"))
  (CallFunction|DeleteGizmo)
  (Utilities|FlowControl|Delay 0.5)
  (Rendering|ExportRenderTarget "/Game/Blueprints/Gizmo/RenderTarget.RenderTarget" _returnvalue_3 _returnvalue_4)
  (bind _returnvalue_5 (Class|KismetRenderingLibrary|ImportFileasTexture2D (Utilities|String|Append _returnvalue_3 _returnvalue_4)))
  (Variables|Default|SetNewVar _returnvalue_5))

(event Custom|setsaveName
  (params (saveName :type Text))
  (Variables|Default|SetsaveName saveName))

(event Custom|addUMG
  (params (W_mainUI :type Widget%20Object%20Reference) (W_inputwindow :type Widget%20Object%20Reference) (W_LIghtAdjust :type Widget%20Object%20Reference))
  (Variables|Default|SetW_mainUI W_mainUI)
  (Variables|Default|SetW_inputwindow W_inputwindow)
  (Variables|Default|SetW_LIghtAdjust W_LIghtAdjust))

(event Custom|clear%20model
  (CallFunction|ClearModel))

(event Custom|lightchange
  (params (value :type Float%20%28double-precision%29)))

(event EventBeginPlay
  (Input|EnableInput (Game|GetPlayerController 0)))

(event EventTick
  (params (DeltaSeconds :type Float%20%28single-precision%29)))

(fn ConstructionScript)

(fn ClearModel
  (bind _outactors (Actor|GetAllActorsOfClass "/Game/Blueprints/TargetAsset/Meshes/BP_TargetStaticmesh.BP_TargetStaticmesh_C"))
  (for _array_element _outactors
    (Actor|DestroyActor _array_element)
    (bind _returnvalue (Actor|GetActorOfClass "/Game/Blueprints/Gizmo/BP_Gizmo.BP_Gizmo_C"))
    (Default|HideGizmo _returnvalue)))

(fn ScreenShot
  (Development|ExecuteConsoleCommand "HighresShot 5000x4000" 0))

(fn DeleteGizmo
  (bind _returnvalue (Actor|GetActorOfClass "/Game/Blueprints/Gizmo/BP_Gizmo.BP_Gizmo_C"))
  (Default|HitorSelectNothing _returnvalue (Variables|/Game/Blueprints/Gizmo/BP_Gizmo.BP_Gizmo_C|GetActorArray _returnvalue)))

(fn Hidewidget
  (params (NewParam :type Widget%20Object%20Reference))
  (Widget|SetVisibility NewParam "Hidden"))

(fn ShowWidget
  (params (NewParam :type Widget%20Object%20Reference))
  (Widget|SetVisibility NewParam "Visible"))

(fn ChangeLight
  (params (Invalue :type Float%20%28double-precision%29))
  (switch int (Variables|Default|GetInclick)
    (:1
      _)
    (:2
      _))
  (for _array_element (Actor|GetComponentsByClass (Variables|Default|GetClickedActor) "/Script/Engine.PointLightComponent")
    (Rendering|Components|Light|SetIntensity _array_element Invalue)))

(fn ChangeColor
  (params (Invalue :type Float%20%28double-precision%29) (InchangePos :type Integer))
  (bind _clickedactor (Variables|Default|GetClickedActor))
  (bind _returnvalue (Actor|GetComponentsByClass _clickedactor "/Script/Engine.PointLightComponent"))
  (bind _output (Utilities|Array|Get(acopy) _returnvalue))
  (bind _returnvalue_2 (Rendering|Components|Light|GetLightColor _output))
  (switch int (Variables|Default|GetInclick)
    (:1
      _)
    (:2
      _))
  (switch int InchangePos
    (:0
      (Rendering|Components|Light|SetLightColor _output (Math|Color|MakeColor Invalue (.g _returnvalue_2) (.b _returnvalue_2) (.a _returnvalue_2)) true))
    (:1
      (Rendering|Components|Light|SetLightColor _output (Math|Color|MakeColor (.r _returnvalue_2) Invalue (.b _returnvalue_2) (.a _returnvalue_2)) true))
    (:2
      (Rendering|Components|Light|SetLightColor _output (Math|Color|MakeColor (.r _returnvalue_2) (.g _returnvalue_2) Invalue (.a _returnvalue_2)) true)))
  (return))

(fn ChangeLightRadio
  (params (Invalue :type Float%20%28double-precision%29))
  (switch int (Variables|Default|GetInclick)
    (:1
      _)
    (:2
      _))
  (for _array_element (Actor|GetComponentsByClass (Variables|Default|GetClickedActor) "/Script/Engine.PointLightComponent")
    (Rendering|Lighting|SetAttenuationRadius _array_element Invalue)))

(fn SetLightSliderValue
  (bind _clickedactor (Variables|Default|GetClickedActor))
  (bind _returnvalue (Actor|GetComponentsByClass _clickedactor "/Script/Engine.PointLightComponent"))
  (bind _output (Utilities|Array|Get(acopy) _returnvalue))
  (bind _lightcolor (Variables|/Script/Engine.LightComponentBase|GetLightColor _output))
  (switch int (Variables|Default|GetInclick)
    (:1
      _)
    (:2
      _))
  (Default|SetValue (.AsW%20Lightadjust (Utilities|Casting|CastToW_Lightadjust (Variables|Default|GetW_LIghtAdjust))) (Variables|/Script/Engine.LightComponentBase|GetIntensity _output) (/ (Math|Conversions|ToFloat(Byte) (.r _lightcolor)) 255.0) (/ (Math|Conversions|ToFloat(Byte) (.g _lightcolor)) 255.0) (/ (Math|Conversions|ToFloat(Byte) (.b _lightcolor)) 255.0) (Variables|/Script/Engine.LocalLightComponent|GetAttenuationRadius _output)))