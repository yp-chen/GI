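; BP_MainPawn is a player-controlled free-moving camera pawn with Enhanced Input movement, look and zoom.
; BeginPlay adds the IMC_MoveBase mapping context; move actions feed AddMovementInput along axes derived from control yaw only.
; Tick polls the right mouse button to gate turning and clamped pitch, while IA_ControlView changes SpringArm length for zoom.
; PreSet is an empty stub, and older SetActorLocation movement logic remains disconnected.
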(event Input|EnhancedActionEvents|EnhancedInputActionIA_ControlView
  (params (ActionValue :type Float%20%28double-precision%29) (ElapsedSeconds :type Float%20%28double-precision%29) (TriggeredSeconds :type Float%20%28double-precision%29) (InputAction :type Input%20Action%20Object%20Reference :default "/Game/Blueprints/Input/IA_ControlView.IA_ControlView"))
  (bind _springarm (Variables|Default|GetSpringArm))
  (:Triggered
    (Variables|/Script/Engine.SpringArmComponent|SetTargetArmLength _springarm (+ (* ActionValue (Variables|Default|GetViewRate)) (Variables|/Script/Engine.SpringArmComponent|GetTargetArmLength _springarm)))))

(event Input|EnhancedActionEvents|EnhancedInputActionIA_MoveForWardOrBack
  (params (ActionValue :type Float%20%28double-precision%29) (ElapsedSeconds :type Float%20%28double-precision%29) (TriggeredSeconds :type Float%20%28double-precision%29) (InputAction :type Input%20Action%20Object%20Reference :default "/Game/Blueprints/Input/IA_MoveForWardOrBack.IA_MoveForWardOrBack"))
  (:Triggered
    (Pawn|Input|AddMovementInput (Math|Vector|GetForwardVector (Math|Rotator|MakeRotator 0.0 0.0 (.yaw (Pawn|GetControlRotation :!class /Script/Engine.Pawn)))) ActionValue false)))

(event Input|EnhancedActionEvents|EnhancedInputActionIA_MoveRightOrLeft
  (params (ActionValue :type Float%20%28double-precision%29) (ElapsedSeconds :type Float%20%28double-precision%29) (TriggeredSeconds :type Float%20%28double-precision%29) (InputAction :type Input%20Action%20Object%20Reference :default "/Game/Blueprints/Input/IA_MoveRightOrLeft.IA_MoveRightOrLeft"))
  (:Triggered
    (Pawn|Input|AddMovementInput (Math|Vector|GetRightVector (Math|Rotator|MakeRotator 0.0 0.0 (.yaw (Pawn|GetControlRotation :!class /Script/Engine.Pawn)))) ActionValue false)))

(event Input|EnhancedActionEvents|EnhancedInputActionIA_TurnRightOrLeft
  (params (ActionValue :type Float%20%28double-precision%29) (ElapsedSeconds :type Float%20%28double-precision%29) (TriggeredSeconds :type Float%20%28double-precision%29) (InputAction :type Input%20Action%20Object%20Reference :default "/Game/Blueprints/Input/IA_TurnRightOrLeft.IA_TurnRightOrLeft"))
  (bind _returnvalue (Pawn|GetControlRotation :!class /Script/Engine.Pawn))
  (:Triggered
    (if (Variables|Default|GetHoldMouseRight)
      (Pawn|SetControlRotation (Pawn|GetController) (Math|Rotator|MakeRotator (.roll _returnvalue) (.pitch _returnvalue) (+ (.yaw _returnvalue) (* ActionValue (Variables|Default|GetRotatoRate))))))))

(event Input|EnhancedActionEvents|EnhancedInputActionIA_LookUpOrDown
  (params (ActionValue :type Float%20%28double-precision%29) (ElapsedSeconds :type Float%20%28double-precision%29) (TriggeredSeconds :type Float%20%28double-precision%29) (InputAction :type Input%20Action%20Object%20Reference :default "/Game/Blueprints/Input/IA_LookUpOrDown.IA_LookUpOrDown"))
  (bind _returnvalue (Pawn|GetControlRotation :!class /Script/Engine.Pawn))
  (:Triggered
    (if (Variables|Default|GetHoldMouseRight)
      (Pawn|SetControlRotation (Pawn|GetController) (Math|Rotator|MakeRotator (.roll _returnvalue) (Math|Float|ClampAngle (+ (.pitch _returnvalue) (* ActionValue (Variables|Default|GetRotatoRate) -1.0)) -7e+01 1e+01) (.yaw _returnvalue))))))

(event Input|EnhancedActionEvents|EnhancedInputActionIA_MoveUpOrDown
  (params (ActionValue :type Float%20%28double-precision%29) (ElapsedSeconds :type Float%20%28double-precision%29) (TriggeredSeconds :type Float%20%28double-precision%29) (InputAction :type Input%20Action%20Object%20Reference :default "/Game/Blueprints/Input/IA_MoveUpOrDown.IA_MoveUpOrDown"))
  (:Triggered
    (Pawn|Input|AddMovementInput (Math|Vector|GetUpVector (Math|Rotator|MakeRotator 0.0 0.0 (.yaw (Pawn|GetControlRotation :!class /Script/Engine.Pawn)))) ActionValue false)))

(event EventBeginPlay
  (bind _returnvalue (Game|GetPlayerController 0))
  (bind _returnvalue_2 (PlayerController|LocalPlayerSubsystems|GetEnhancedInputLocalPlayerSubsystem _returnvalue))
  (Utilities|IsValid _returnvalue_2
    (:Is%20Valid
      (Input|AddMappingContext _returnvalue_2 "/Game/Blueprints/Input/IMC_MoveBase.IMC_MoveBase" 0 "(bIgnoreAllPressedKeysUntilRelease=True,bForceImmediately=False,bNotifyUserSettings=False)"))))

(event EventTick
  (params (DeltaSeconds :type Float%20%28single-precision%29))
  (Variables|Default|SetHoldMouseRight (Game|Player|IsInputKeyDown (Game|GetPlayerController 0) "RightMouseButton")))

(fn ConstructionScript)

(fn PreSet
  (params (Condition :type Boolean))
  (if Condition
    _))