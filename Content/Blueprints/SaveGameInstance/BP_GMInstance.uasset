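; Game instance that saves and loads placed target meshes and their lights in a named slot.
; Saving replaces the slot with a new BP_SaveGame filled with indices, transforms and light info from the first BP_Gizmo.
; Loading clears models via TargetGameMode, then respawns BP_TargetStaticmesh actors with collision.
; Spot or point lights are added at runtime and configured through their shared PointLightComponent class.
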(fn GetAllTargetMesh
  ;[0.15 0.15 0.15 0.5] 调用gizmo的保存游戏的函数获取游戏保存数据
  (bind _outactors (Actor|GetAllActorsOfClass "/Game/Blueprints/Gizmo/BP_Gizmo.BP_Gizmo_C"))
  (Utilities|IsValid (Utilities|Array|Get(acopy) _outactors)
    (:Is%20Valid
      (bind (_targetlistindex _targettransform _removeransform _lightsaveinfo) (Default|SaveGameRef (Utilities|Array|Get(acopy) _outactors)))
      (return _targetlistindex _targettransform _removeransform _lightsaveinfo))))

(fn SaveGameRef
  (bind _slot_name (Variables|SaveGame|GetSlot%20Name))
  ;[0.15 0.15 0.15 0.5] 根据slotname新建savegame，并保存游戏数据
  (bind _returnvalue (SaveGame|DoesSaveGameExist _slot_name))
  (if _returnvalue
    (bind _returnvalue_2 (SaveGame|DeleteGameinSlot _slot_name))
    (if _returnvalue_2
      (bind _returnvalue_3 (SaveGame|CreateSaveGameObject "/Game/Blueprints/SaveGameInstance/BP_SaveGame.BP_SaveGame_C" :!label _label))
      (Variables|SaveGame|SetSaveGameIns _returnvalue_3)
      (SaveGame|SaveTargetMesh))
    (else
      (goto _label))))

(fn SaveTargetMesh
  (bind _savegameins (Variables|SaveGame|GetSaveGameIns))
  (bind _savegameins_2 (Variables|SaveGame|GetSaveGameIns))
  ;[0.15 0.15 0.15 0.5] 清空原有数据
  (Utilities|IsValid _savegameins
    (:Is%20Valid
      (Utilities|Array|Clear (Variables|/Game/Blueprints/SaveGameInstance/BP_SaveGame.BP_SaveGame_C|GetTransformVector _savegameins))
      (Utilities|Array|Clear (Variables|/Game/Blueprints/SaveGameInstance/BP_SaveGame.BP_SaveGame_C|GetTargetListIndex _savegameins))
      (bind (_targetlistindex _targettransform _removeransform _lightsaveinfo) (SaveGame|GetAllTargetMesh))
      (Variables|/Game/Blueprints/SaveGameInstance/BP_SaveGame.BP_SaveGame_C|SetTargetListIndex _savegameins_2 _targetlistindex)
      (Variables|/Game/Blueprints/SaveGameInstance/BP_SaveGame.BP_SaveGame_C|SetTransformVector _savegameins_2 _targettransform)
      (Variables|/Game/Blueprints/SaveGameInstance/BP_SaveGame.BP_SaveGame_C|SetLightSaveInfo _savegameins_2 _lightsaveinfo)
      (bind _returnvalue (SaveGame|SaveGametoSlot _savegameins_2 (Variables|SaveGame|GetSlot%20Name)))
      (if _returnvalue
        _))))

(fn LoadGameRef
  (bind _slot_name (Variables|SaveGame|GetSlot%20Name))
  (bind _returnvalue (SaveGame|DoesSaveGameExist _slot_name))
  (if _returnvalue
    (bind _returnvalue_2 (SaveGame|LoadGamefromSlot _slot_name))
    (bind _asbp_save_game (Utilities|Casting|CastToBP_SaveGame _returnvalue_2))
    (LoadGame|LoadTargetInfo _asbp_save_game)))

(fn LoadTargetInfo
  (params (SaveTarget :type BP%20Save%20Game%20Object%20Reference))
  (Default|ClearModel (.AsTarget%20Game%20Mode (Utilities|Casting|CastToTargetGameMode (Game|GetGameMode))))
  (for (_array_element _array_index) (Variables|/Game/Blueprints/SaveGameInstance/BP_SaveGame.BP_SaveGame_C|GetTargetListIndex SaveTarget)
    (bind _returnvalue (Game|SpawnActorfromClass "/Game/Blueprints/TargetAsset/Meshes/BP_TargetStaticmesh.BP_TargetStaticmesh_C" (Utilities|Array|Get(acopy) (Variables|/Game/Blueprints/SaveGameInstance/BP_SaveGame.BP_SaveGame_C|GetTransformVector SaveTarget) _array_index) "Undefined" "MultiplyWithRoot" 0 _array_element 0))
    (Collision|SetCollisionEnabled (Variables|/Script/Engine.StaticMeshActor|GetStaticMeshComponent _returnvalue) "QueryAndPhysics")
    (bind _output_get (LocalVariables|SetTempActor _returnvalue))
    (CallFunction|SetLightInfo _output_get (Utilities|Array|Get(acopy) (Variables|/Game/Blueprints/SaveGameInstance/BP_SaveGame.BP_SaveGame_C|GetLightSaveInfo SaveTarget) _array_index)))
  (return))

(fn Setslotname
  (params (Inslotname :type Text))
  (Variables|SaveGame|SetSlot%20Name (Utilities|String|ToString(Text) Inslotname)))

(fn SetLightInfo
  (params (Actor :type BP%20Target%20Staticmesh%20Object%20Reference) (LightInfo :type Light%20Save%20Info%20Structure))
  (bind (_haspoint _hasspot _intensity _r _g _b _radio) (Utilities|Struct|BreakLightSaveInfo LightInfo))
  (bind _returnvalue (Actor|GetComponentsByClass Actor "/Script/Engine.PointLightComponent"))
  (bind _output (Utilities|Array|Get(acopy) _returnvalue))
  (if _hasspot
    (Game|AddComponentbyClass Actor "/Script/Engine.SpotLightComponent" false)
    (Rendering|Components|Light|SetIntensity _output (.intensity LightInfo) :!label _label)
    (Rendering|Components|Light|SetLightColor _output (Math|Color|MakeColor (/ (.r LightInfo) 255.0) (/ (.g LightInfo) 255.0) (/ (.b LightInfo) 255.0)) true)
    (Rendering|Lighting|SetAttenuationRadius _output _radio)
    (elif _haspoint
      (Game|AddComponentbyClass Actor "/Script/Engine.PointLightComponent" false)
      (goto _label))))